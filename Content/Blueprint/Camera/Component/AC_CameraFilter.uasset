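; Camera filter component that switches UV, thermal and audio visual filters through post-process materials.
; On BeginPlay it waits for the scene manager to initialize, then caches managers and the post-process volume and binds to the camera manager's filter-change event.
; Each change sets the current material's weight to full and zeroes the previously stored one, skipping two reserved indices, then stores the new index.
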(event `self.ReceiveBeginPlay`
  (bind _output_get (set `self.Scene Manager` (`/Game/Blueprint/Global/BFL_FunctionEverywhere.InitiateSceneManager`)))
  (add `/Game/Blueprint/Global/Manager/BP_SceneManager.OnInitiateManagerEvent` _output_get (delegate `Initialization_Event`)))

(event `Initialization_Event`
  (`|ExecutionSequence`
    (:`then_0`
      (`self.SetManagerVariable`))
    (:`then_1`
      (`self.BindAllEvent`))))

(event `BindFilterEvent`
  (bind _camera_actor_manager (`self.Camera Actor Manager`))
  ;[0.102 0.2196 1] Filter Change Event
  (add `/Game/Blueprint/Global/Manager/BP_CameraActorManager.OnChangeFilter` _camera_actor_manager (delegate `ChangeFIlter`))
  (`self.GetPostProcessVolume` _camera_actor_manager))

(event `ChangeFIlter`
  (params (ESelectedFilter :type "/Game/Data/Enumerator/Camera/ECameraFilter Enum" :default "NewEnumerator0") (PostProcessIndex :type Integer))
  ;[0.102 0.2196 1] Filter Change Event
  (`self.HandleFilterVisual` ESelectedFilter PostProcessIndex))

(fn `BindAllEvent`
  (`self.BindFilterEvent`))

(fn `DisableFilterVisual`
  (params (`PostProcess Index` :type Integer) (Item_Weight :type "Float (single-precision)"))
  (`self.SetPostprocessElement` `PostProcess Index` Item_Weight (`.Array` (break `WeightedBlendables` (`.WeightedBlendables` (break `PostProcessSettings` (`PostProcessVolume.Settings` (`self.Post Process Scene`))))))))

(fn `EnableFilterVisual`
  (params (`PostProcess Index` :type Integer) (`Filter Visual Weight` :type "Float (single-precision)"))
  (`self.SetPostprocessElement` `PostProcess Index` `Filter Visual Weight` (`.Array` (break `WeightedBlendables` (`.WeightedBlendables` (break `PostProcessSettings` (`PostProcessVolume.Settings` (`self.Post Process Scene`))))))))

(fn `GetPostProcessVolume`
  (params (`Camera Manager` :type "/Game/Blueprint/Global/Manager/BP_CameraActorManager Object Reference"))
  (set `self.Post Process Scene` (`/Game/Blueprint/Global/Manager/BP_CameraActorManager.PostProcess` `Camera Manager`)))

(fn `HandleFilterVisual`
  (params (EFilterVisual :type "/Game/Data/Enumerator/Camera/ECameraFilter Enum" :default "NewEnumerator0") (`Index PostProcess` :type Integer))
  (locals (`Current Filter` :type "/Game/Data/Enumerator/Camera/ECameraFilter Enum" :default "NewEnumerator0"))
  (bind _filterpostprocess (`self.FilterPostProcess`))
  (bind _current_postprocess_index (`/Game/Blueprint/Global/Manager/BP_CameraActorManager.Current PostProcess Index` (`self.Camera Actor Manager`)))
  (`|ExecutionSequence`
    (:`then_0`
      (switch `/Game/Data/Enumerator/Camera/ECameraFilter` EFilterVisual
        (:`NewEnumerator0`
          _)
        (:`NewEnumerator1`
          (`self.EnableFilterVisual` _current_postprocess_index 1.0))
        (:`NewEnumerator2`
          (`self.EnableFilterVisual` _current_postprocess_index 1.0))
        (:`NewEnumerator3`
          (`self.EnableFilterVisual` _current_postprocess_index 1.0)))
      (if (and (!= _filterpostprocess 0) (!= _filterpostprocess 4) (!= _filterpostprocess _current_postprocess_index))
        (`self.DisableFilterVisual` (`self.FilterPostProcess`))))
    (:`then_1`
      (set `self.FilterPostProcess` `Index PostProcess`))))

(fn `SetManagerVariable`
  (bind _scene_manager (`self.Scene Manager`))
  (set `self.Camera Actor Manager` (`/Game/Blueprint/Global/Manager/BP_SceneManager.CameraActorManager` _scene_manager))
  (set `self.Hint Manager` (`/Game/Blueprint/Global/Manager/BP_SceneManager.HintManager` _scene_manager)))

(fn `SetPostprocessElement`
  (params (Index :type Integer) (Item_Weight :type "Float (single-precision)") (Array :type "Array of WeightedBlendable Structure"))
  (bind (_output_weight _output_object) (break `WeightedBlendable` (`|GetArrayItem` Array Index)))
  (`KismetArrayLibrary.Array_Set` Array Index (make `WeightedBlendable` Item_Weight _output_object)))