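; BP_SceneManager is a scene manager that gathers references to the game's singleton managers and triggers their initialization event at startup.
; On BeginPlay it casts and caches the Data, Hint, CameraActor, Sequencer, UI, Computer and GameState managers through GetSingletonInstance.
; After a half-second delay it calls CallOnInitiateManagerEvent.
; A failed cast skips the remaining lookups in that sequence branch.
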(event `self.ReceiveBeginPlay`
  (`|ExecutionSequence`
    (:`then_0`
      (`self.GetSingletonManager`))
    (:`then_1`
      (`KismetSystemLibrary.Delay` 0.5)
      (`self.OnInitiateManagerEvent`))))

(fn `GetSingletonManager`
  (`|ExecutionSequence`
    (:`then_0`
      (bind _asbp_data_manager (cast `/Game/Blueprint/Global/Manager/BP_DataManager` (`/Game/Blueprint/Global/BFL_FunctionEverywhere.GetSingletonInstance` "/Game/Blueprint/Global/Manager/BP_DataManager.BP_DataManager_C")))
      (set `self.DataManager` _asbp_data_manager)
      (bind _asbp_hint_manager (cast `/Game/Blueprint/Global/Manager/BP_HintManager` (`/Game/Blueprint/Global/BFL_FunctionEverywhere.GetSingletonInstance` "/Game/Blueprint/Global/Manager/BP_HintManager.BP_HintManager_C")))
      (set `self.HintManager` _asbp_hint_manager))
    (:`then_1`
      (bind _asbp_camera_actor_manager (cast `/Game/Blueprint/Global/Manager/BP_CameraActorManager` (`/Game/Blueprint/Global/BFL_FunctionEverywhere.GetSingletonInstance` "/Game/Blueprint/Global/Manager/BP_CameraActorManager.BP_CameraActorManager_C")))
      (set `self.CameraActorManager` _asbp_camera_actor_manager)
      (bind _asbp_sequencer_manager (cast `/Game/Blueprint/Global/Manager/BP_SequencerManager` (`/Game/Blueprint/Global/BFL_FunctionEverywhere.GetSingletonInstance` "/Game/Blueprint/Global/Manager/BP_SequencerManager.BP_SequencerManager_C")))
      (set `self.SequencerManager` _asbp_sequencer_manager))
    (:`then_2`
      (bind _asbp_uimanager (cast `/Game/Blueprint/Global/Manager/BP_UIManager` (`/Game/Blueprint/Global/BFL_FunctionEverywhere.GetSingletonInstance` "/Game/Blueprint/Global/Manager/BP_UIManager.BP_UIManager_C")))
      (set `self.UIManager` _asbp_uimanager)
      (bind _asbp_computer_manager (cast `/Game/Blueprint/Global/Manager/BP_ComputerManager` (`/Game/Blueprint/Global/BFL_FunctionEverywhere.GetSingletonInstance` "/Game/Blueprint/Global/Manager/BP_ComputerManager.BP_ComputerManager_C")))
      (set `self.ComputerManager` _asbp_computer_manager)
      (bind _asbp_game_state_manager (cast `/Game/Blueprint/Global/Manager/BP_GameStateManager` (`/Game/Blueprint/Global/BFL_FunctionEverywhere.GetSingletonInstance` "/Game/Blueprint/Global/Manager/BP_GameStateManager.BP_GameStateManager_C")))
      (set `self.GameStateManager` _asbp_game_state_manager))))

(fn `UserConstructionScript`)