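; BP_DataManager is a manager that stores the hint and citizen data found so far, keyed by hint name.
; On BeginPlay it waits for the scene manager's initiate event, then hands itself to its hint and citizen data components and has both bind their events.
; Each add call updates the matching map, then broadcasts both maps and the hint name through OnSendData.
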(event `AddCitizenData`
  (params (HintName :type Name) (CitizenData :type "/Game/Data/Stucture/Citizen/SCitizenData Structure"))
  ;[1 1 1] Tempon Data
  (`BlueprintMapLibrary.Map_Add` (`self.CitizenDataAlreadyFind`) HintName CitizenData)
  (`self.OnSendData` (`self.CitizenDataAlreadyFind`) (`self.HintDataAlreadyFind`) HintName :!label _label))

(event `self.ReceiveBeginPlay`
  ;[1 1 1] Initialization Event
  (`self.BindInitiate`))

(event `AddHintData`
  (params (HintName :type Name) (HintData :type "/Game/Data/Stucture/Hint/SHintData Structure"))
  ;[1 1 1] Tempon Data
  (`BlueprintMapLibrary.Map_Add` (`self.HintDataAlreadyFind`) HintName HintData)
  (goto _label))

(event `BindInitiate`
  ;[1 1 1] Initialization Event
  (bind _output_get (set `self.Scene Manager` (`/Game/Blueprint/Global/BFL_FunctionEverywhere.InitiateSceneManager`)))
  (add `/Game/Blueprint/Global/Manager/BP_SceneManager.OnInitiateManagerEvent` _output_get (delegate `OnInitiateManagerEvent_Event`)))

(event `OnInitiateManagerEvent_Event`
  ;[1 1 1] Initialization Event
  (`|ExecutionSequence`
    (:`then_0`
      (`self.SetAllManagerVariable`))
    (:`then_1`
      (`self.BindAllEvent`))))

(fn `BindAllEvent`
  (`/Game/Blueprint/Data/Component/AC_DataController.BindAllEvent` (`self.AC_HintData`))
  (`/Game/Blueprint/Data/Component/AC_DataController.BindAllEvent` (`self.AC_CitizenData`)))

(fn `SetAllManagerVariable`
  (set `/Game/Blueprint/Data/Component/AC_DataController.DataManager` self (`self.AC_HintData`))
  (set `/Game/Blueprint/Data/Component/AC_DataController.DataManager` self (`self.AC_CitizenData`)))

(fn `UserConstructionScript`)