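; BP_HUBScreen is the office screen controller that shows and removes the hub widget through the UI manager.
; Once the scene manager initiates, it caches the UI and Data managers, binds events and registers itself on the widget.
; Research and sent-data events look up citizens by name to fill the Data Center panel.
; Analysis report, timed popup and map ping handlers exist, but their bindings are empty or disconnected.
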(event `self.ReceiveBeginPlay`
  ;[0.04911 0.6101 1] Initialization Binding Event
  (`self.BindInitiate`))

(event `BindInitiate`
  ;[0.04911 0.6101 1] Initialization Binding Event
  (bind _output_get (set `self.Scene Manager` (`/Game/Blueprint/Global/BFL_FunctionEverywhere.InitiateSceneManager`)))
  (add `/Game/Blueprint/Global/Manager/BP_SceneManager.OnInitiateManagerEvent` _output_get (delegate `Initiate Event`)))

(event `DisplayHubWidget`
  (bind _uimanager (`self.UIManager`))
  ;[1 1 1] Display/Remove Widget
  (`/Game/Blueprint/Global/Manager/BP_UIManager.DisplayWidget` _uimanager true (`/Game/Blueprint/Global/Manager/BP_UIManager.HubScreen` _uimanager)))

(event `Initiate Event`
  ;[0.04911 0.6101 1] Initialization Binding Event
  (`|ExecutionSequence`
    (:`then_0`
      (`self.SetManagerVariable`))
    (:`then_1`
      (`self.BindAllEvent`))
    (:`then_2`
      (set `/Game/Widget/HUBScreen/WBP_HUBScreen.HUBScreenController` self (`/Game/Blueprint/Global/Manager/BP_UIManager.HubScreen` (`self.UIManager`))))))

(event `RemoveHubWidget`
  (bind _uimanager (`self.UIManager`))
  ;[1 1 1] Display/Remove Widget
  (`/Game/Blueprint/Global/Manager/BP_UIManager.RemoveWidget` _uimanager (`/Game/Blueprint/Global/Manager/BP_UIManager.HubScreen` _uimanager)))

(event `BindArchiveSelected`
  ;[0.6146 0 0.02394] ??????
)

(event `OnAnalyseSelect_Event`
  (params (HintSelect :type "/Game/Blueprint/Hint/BP_AHintController Object Reference"))
  ;[0.6146 0 0.02394] ??????
  (`MenuAnchor.Open` (`/Game/Widget/HUBScreen/WBP_HUBScreen.Popup` (`/Game/Blueprint/Global/Manager/BP_UIManager.HubScreen` (`self.UIManager`))) false)
  (`KismetSystemLibrary.K2_SetTimerDelegate` (delegate `CustomEvent`) 5.0))

(event `CustomEvent`
  ;[0.6146 0 0.02394] ??????
  (`MenuAnchor.Close` (`/Game/Widget/HUBScreen/WBP_HUBScreen.Popup` (`/Game/Blueprint/Global/Manager/BP_UIManager.HubScreen` (`self.UIManager`)))))

(event `ArchiveSelected_Event`
  (params (bIsSelected :type Boolean))
  ;[0.6146 0 0.02394] ??????
)

(event `BindAnalyseInProgress`
  ;[0.04911 0.6101 1] Analyse Report
)

(event `AnalyseInProgress_Event`
  (params (CurrentHint :type "/Game/Blueprint/Data/Component/AC_DataController Object Reference") (HintElement :type "/Game/Data/Stucture/Hint/SHintNoFilterData Structure") (UVHint :type "/Game/Data/Stucture/Hint/SHintUVData Structure") (Image :type "Texture2D Object Reference"))
  ;[0.04911 0.6101 1] Analyse Report
  (`/Game/Widget/HUBScreen/AnalysisReport/WBP_AnalysisReport.GetCurrentHint` :`self` (`/Game/Widget/HUBScreen/WBP_HUBScreen.WBP_AnalysisReport` (`/Game/Blueprint/Global/Manager/BP_UIManager.HubScreen` (`self.UIManager`)))))

(event `BindDisplayResearch`
  ;[1 1 1] Research result display on data center
  (add `/Game/Blueprint/Global/Manager/BP_UIManager.OnDisplayResearch` (`self.UIManager`) (delegate `DisplayResearch_Event`))
  (add `/Game/Blueprint/Global/Manager/BP_DataManager.OnSendData` (`self.Data Manager`) (delegate `BindSendData`)))

(event `DisplayResearch_Event`
  (params (CitizenName :type Name))
  ;[1 1 1] Research result display on data center
  (`self.ViewCitizenData` (`/Game/Blueprint/Global/Manager/BP_DataManager.CitizenDataAlreadyFind` (`self.Data Manager`)) CitizenName))

(event `BindSendData`
  (params (CitizenData :type "Map of Name to /Game/Data/Stucture/Citizen/SCitizenData Structure") (HintData :type "Map of Name to /Game/Data/Stucture/Hint/SHintData Structure") (HintName :type Name))
  ;[1 1 1] Research result display on data center
  (`self.ViewCitizenData` CitizenData HintName))

(event `BindClicked`)

(event `Click_Event`
  (`/Game/Widget/HUBScreen/MapDallas/WBP_DallasMap.DisplaySuspectPing` (`/Game/Widget/HUBScreen/WBP_HUBScreen.WBP_Map` (`/Game/Blueprint/Global/Manager/BP_UIManager.HubScreen` (`self.UIManager`)))))

(event `SuspectPing`
  (params (Suspect :type Name))
  (set `/Game/Widget/HUBScreen/MapDallas/WBP_DallasMap.Suspect` Suspect (`/Game/Widget/HUBScreen/WBP_HUBScreen.WBP_Map` (`/Game/Blueprint/Global/Manager/BP_UIManager.HubScreen` (`self.UIManager`)))))

(fn `BindAllEvent`
  (`self.BindAnalyseInProgress`)
  (`self.BindClicked`)
  (`self.BindDisplayResearch`)
  (`self.BindArchiveSelected`))

(fn `SetManagerVariable`
  (locals (NewLocalVar :type "/Game/Blueprint/Global/Manager/BP_SceneManager Object Reference"))
  (bind _scene_manager (`self.Scene Manager`))
  (set `self.UIManager` (`/Game/Blueprint/Global/Manager/BP_SceneManager.UIManager` _scene_manager))
  (set `self.Data Manager` (`/Game/Blueprint/Global/Manager/BP_SceneManager.DataManager` _scene_manager)))

(fn `UserConstructionScript`)

(fn `ViewCitizenData`
  (params (CitizenData :type "Map of Name to /Game/Data/Stucture/Citizen/SCitizenData Structure (by ref)") (`Citizen Name` :type Name))
  (bind (_value _returnvalue) (`BlueprintMapLibrary.Map_Find` CitizenData `Citizen Name`))
  (bind _wbp_datacenter (`/Game/Widget/HUBScreen/WBP_HUBScreen.WBP_DataCenter` (`/Game/Blueprint/Global/Manager/BP_UIManager.HubScreen` (`self.UIManager`))))
  (if _returnvalue
    (`/Game/Widget/HUBScreen/InformationsCenter/WBP_DataCenter.GetSearchData` _wbp_datacenter _value)
    (`/Game/Widget/HUBScreen/InformationsCenter/WBP_DataCenter.Add Result Button` _wbp_datacenter `Citizen Name`)))