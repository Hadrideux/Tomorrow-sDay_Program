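; BP_SequencerController applies playback state, time and speed changes from the SequencerManager to its current Level Sequence.
; On BeginPlay it waits for the SceneManager's initiate event, then caches the SequencerManager and binds to its state, timecode and speed delegates.
; The handlers play or pause the sequence, jump to the given time while storing it on the manager, or set one of three play rates.
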(event `self.ReceiveBeginPlay`
  ;[1 1 1] Initialization Binding Event
  (bind _output_get (set `self.Scene Manager` (`/Game/Blueprint/Global/BFL_FunctionEverywhere.InitiateSceneManager`)))
  (add `/Game/Blueprint/Global/Manager/BP_SceneManager.OnInitiateManagerEvent` _output_get (delegate `Initialization_Event`)))

(event `Initialization_Event`
  ;[1 1 1] Initialization Binding Event
  (`|ExecutionSequence`
    (:`then_0`
      (`self.SetManagerVariable`))
    (:`then_1`
      (`self.BindAllEvent`))))

(event `BindSequenceState`
  ;[1 0.1311 0.07812] Play/Pause Sequence
  (add `/Game/Blueprint/Global/Manager/BP_SequencerManager.OnSequenceStateChange` (`self.SequencerManager`) (delegate `SequenceState_Event`)))

(event `BindSequencerTime`
  ;[0.2672 1 0.1234] TimeCode Sequence
  (add `/Game/Blueprint/Global/Manager/BP_SequencerManager.OnChangeTimeCode` (`self.SequencerManager`) (delegate `OnChangeTimeCcode`)))

(event `BindSequenceSpeed`
  (add `/Game/Blueprint/Global/Manager/BP_SequencerManager.OnSequenceSpeedChange` (`self.SequencerManager`) (delegate `SequenceSpeed_Event`)))

(event `OnChangeTimeCcode`
  (params (`Sequence Time` :type "Float (double-precision)"))
  (bind _sequencermanager (`self.SequencerManager`))
  ;[0.2672 1 0.1234] TimeCode Sequence
  (bind _output_get (set `/Game/Blueprint/Global/Manager/BP_SequencerManager.Sequence Playback Time` `Sequence Time` _sequencermanager))
  (`MovieSceneSequencePlayer.SetPlaybackPosition` (`/Game/Blueprint/Global/Manager/BP_SequencerManager.Current Level Sequence` _sequencermanager) (make `MovieSceneSequencePlaybackParams` (make `FrameTime` (make `FrameNumber` (`KismetMathLibrary.FTrunc` _output_get))) _output_get "" "Frame" "Jump")))

(event `SequenceSpeed_Event`
  (params (`Sequencer Speed` :type "/Game/Data/Enumerator/State/ESequencerSpeed Enum" :default "NewEnumerator0"))
  (bind _current_level_sequence (`/Game/Blueprint/Global/Manager/BP_SequencerManager.Current Level Sequence` (`self.SequencerManager`)))
  (switch `/Game/Data/Enumerator/State/ESequencerSpeed` `Sequencer Speed`
    (:`NewEnumerator0`
      (`MovieSceneSequencePlayer.SetPlayRate` _current_level_sequence 0.5))
    (:`NewEnumerator1`
      (`MovieSceneSequencePlayer.SetPlayRate` _current_level_sequence 1.0))
    (:`NewEnumerator2`
      (`MovieSceneSequencePlayer.SetPlayRate` _current_level_sequence 2.0))))

(event `SequenceState_Event`
  (params (SequencerState :type "/Game/Data/Enumerator/State/ESequencerState Enum" :default "NewEnumerator0"))
  (bind _current_level_sequence (`/Game/Blueprint/Global/Manager/BP_SequencerManager.Current Level Sequence` (`self.SequencerManager`)))
  ;[1 0.1311 0.07812] Play/Pause Sequence
  (switch `/Game/Data/Enumerator/State/ESequencerState` SequencerState
    (:`NewEnumerator1`
      (`MovieSceneSequencePlayer.Play` _current_level_sequence))
    (:`NewEnumerator2`
      (`MovieSceneSequencePlayer.Pause` _current_level_sequence))))

(fn `BindAllEvent`
  (`self.BindSequencerTime`)
  (`self.BindSequenceState`)
  (`self.BindSequenceSpeed`))

(fn `SetManagerVariable`
  (set `self.SequencerManager` (`/Game/Blueprint/Global/Manager/BP_SceneManager.SequencerManager` (`self.Scene Manager`))))

(fn `UserConstructionScript`)