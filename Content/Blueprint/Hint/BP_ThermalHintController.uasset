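; BP_ThermalHintController is a hint controller, named for a thermal hint, that listens for filter visual activation from the HintManager.
; On BeginPlay it waits for the SceneManager's manager-initiation event, then sets its manager variables and binds its events.
; The filter handler switches on the EActiveFilter value, but no case has any logic wired yet.
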(event `self.ReceiveBeginPlay`
  ;[1 1 1] Initialization Binding Event
  (`self.Initiate`))

(event `Initiate`
  ;[1 1 1] Initialization Binding Event
  (bind _output_get (set `self.Scene Manager` (`/Game/Blueprint/Global/BFL_FunctionEverywhere.InitiateSceneManager`)))
  (add `/Game/Blueprint/Global/Manager/BP_SceneManager.OnInitiateManagerEvent` _output_get (delegate `Initialization_Event`)))

(event `Initialization_Event`
  ;[1 1 1] Initialization Binding Event
  (`|ExecutionSequence`
    (:`then_0`
      (`self.SetManagerVariable`))
    (:`then_1`
      (`self.Bind All Event`))))

(event `BindActiveFilter`
  (add `/Game/Blueprint/Global/Manager/BP_HintManager.OnEnableFilterVisual` (`self.Hint Manager`) (delegate `ActiveFilter_Event`)))

(event `ActiveFilter_Event`
  (params (EActiveFilter :type "/Game/Data/Enumerator/Camera/ECameraFilter Enum" :default "NewEnumerator0"))
  (switch `/Game/Data/Enumerator/Camera/ECameraFilter` EActiveFilter))

(fn `Bind All Event`
  (`self.BindActiveFilter`))

(fn `UserConstructionScript`)