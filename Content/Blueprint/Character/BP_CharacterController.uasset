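; First-person desk-view player with clamped look angles, FOV zoom and selection of desk elements.
; Once the scene manager initiates, it caches the TomorrowsDay player controller and binds to its look and interact events.
; Looking adds yaw and pitch, then line-traces from the camera to outline the focused desk element or fax through custom depth.
; Interacting with a traced desk element asks the player controller to switch possession to its OfficeElement.
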(event `self.ReceiveBeginPlay`
  ;[0.09237 0.518 1 1 25] Initialization
  (`self.BindInitiate`))

(event `BindInitiate`
  ;[0.09237 0.518 1 1 25] Initialization
  (bind _output_get (set `self.Scene Manager` (`/Game/Blueprint/Global/BFL_FunctionEverywhere.InitiateSceneManager`)))
  (add `/Game/Blueprint/Global/Manager/BP_SceneManager.OnInitiateManagerEvent` _output_get (delegate `Initate`)))

(event `Initate`
  ;[0.09237 0.518 1 1 25] Initialization
  (`|ExecutionSequence`
    (:`then_0`
      (`self.SetManagerVariable`))
    (:`then_1`
      (`self.BindAllEvent`))))

(event `BindLookAt_Event`
  ;[0.09237 0.518 1 1 25] Look
  (add `/Game/Blueprint/Global/BP_TomorrowsDay_PC.OnLookAt` (`self.Tomorrows Day PC`) (delegate `LookAt_Event`)))

(event `LookAt_Event`
  (params (`LookAt Value` :type "Vector2D Structure"))
  ;[0.09237 0.518 1 1 25] Look
  (`|ExecutionSequence`
    (:`then_0`
      (`self.AddControllerYawInput` `LookAt Value_X`))
    (:`then_1`
      (`self.AddControllerPitchInput` `LookAt Value_Y`)))
  (`self.FocusOutline`))

(event `EnhancedInput|/Game/Blueprint/Character/Input/Action/Game/Player/IA_Zoom`
  (params (ActionValue :type Boolean) (ElapsedSeconds :type "Float (double-precision)") (TriggeredSeconds :type "Float (double-precision)") (InputAction :type "InputAction Object Reference" :default "/Game/Blueprint/Character/Input/Action/Game/Player/IA_Zoom.IA_Zoom"))
  ;[0.09237 0.518 1 1 25] Zoom
  (:`Started`
    (bind (_direction _zoom) (`Timeline|Zoom` :!label _label)
      (:`Update`
        (`CameraComponent.SetFieldOfView` (`self.Camera`) (`KismetMathLibrary.Lerp` 90.0 45.0 _zoom)))))
  (:`Completed`
    (goto _label :!via `Reverse`)))

(event `BindPlayerInteract_Event`
  ;[1 1 1] Ajouté Fax et radio en élément
  (add `/Game/Blueprint/Global/BP_TomorrowsDay_PC.OnPlayerInteract` (`self.Tomorrows Day PC`) (delegate `OnPlayerInteract_Event`)))

(event `OnPlayerInteract_Event`
  ;[1 1 1] Ajouté Fax et radio en élément
  (bind _hitactor (`self.ObjectSelection` "TraceTypeQuery3"))
  (bind _asbp_desk_element (cast `/Game/Blueprint/Office/BP_DeskElement` _hitactor))
  (`/Game/Blueprint/Global/BP_TomorrowsDay_PC.OnChangePossesPawn` (`self.Tomorrows Day PC`) (`/Game/Blueprint/Office/BP_DeskElement.OfficeElement` _asbp_desk_element)))

(fn `BindAllEvent`
  (`self.BindLookAt_Event`)
  (`self.BindPlayerInteract_Event`))

(fn `ContraintViewAngle`
  (bind _returnvalue (`GameplayStatics.GetPlayerCameraManager` 0))
  (bind (_returnvalue_roll _returnvalue_pitch _returnvalue_yaw) (`KismetMathLibrary.BreakRotator` (`SceneComponent.K2_GetComponentRotation` (`self.Camera`))))
  (bind (_returnvalue_roll_2 _returnvalue_pitch_2 _returnvalue_yaw_2) (`KismetMathLibrary.BreakRotator` (`SceneComponent.K2_GetComponentRotation` (`self.Camera`))))
  (`|ExecutionSequence`
    (:`then_0`
      (set `PlayerCameraManager.ViewPitchMax` (+ (`self.PitchValue`) _returnvalue_pitch_2) _returnvalue)
      (set `PlayerCameraManager.ViewYawMax` (+ (`self.YawValue`) _returnvalue_yaw_2) _returnvalue))
    (:`then_1`
      (set `PlayerCameraManager.ViewPitchMin` (- _returnvalue_pitch (`self.PitchValue`)) _returnvalue)
      (set `PlayerCameraManager.ViewYawMin` (- _returnvalue_yaw (`self.YawValue`)) _returnvalue))))

(fn `DisplayCrosshair`
  (bind _returnvalue (`|CreateWidget` "/Game/Widget/Misc/WBP_Crosshair.WBP_Crosshair_C"))
  (`UserWidget.AddToViewport` _returnvalue 0))

(fn `FocusOutline`
  (bind _current_desk_element_focused (`self.Current Desk Element Focused`))
  (bind _focusfax (`self.FocusFax`))
  (`|ExecutionSequence`
    (:`then_0`
      (`/Engine/EditorBlueprintResources/StandardMacros.IsValid` _current_desk_element_focused
        (:`Is Valid`
          (`PrimitiveComponent.SetRenderCustomDepth` (`/Game/Blueprint/Office/BP_DeskElement.StaticMesh` _current_desk_element_focused) false))
        (:`Is Not Valid`
          _))
      (bind _hitactor (`self.ObjectSelection` (`self.Trace Channel`)))
      (bind _asbp_desk_element (cast `/Game/Blueprint/Office/BP_DeskElement` _hitactor))
      (`PrimitiveComponent.SetRenderCustomDepth` (`/Game/Blueprint/Office/BP_DeskElement.StaticMesh` _asbp_desk_element) true)
      (set `self.Current Desk Element Focused` _asbp_desk_element))
    (:`then_1`
      (`/Engine/EditorBlueprintResources/StandardMacros.IsValid` _focusfax
        (:`Is Valid`
          (`PrimitiveComponent.SetRenderCustomDepth` (`/Game/Blueprint/Office/BP_Fax.Fax` _focusfax) false))
        (:`Is Not Valid`
          _))
      (bind _hitactor_2 (`self.ObjectSelection` (`self.Trace Channel`)))
      (bind _asbp_fax (cast `/Game/Blueprint/Office/BP_Fax` _hitactor_2))
      (`PrimitiveComponent.SetRenderCustomDepth` (`/Game/Blueprint/Office/BP_Fax.Fax` _asbp_fax) true)
      (set `self.FocusFax` _asbp_fax))))

(fn `ObjectSelection`
  (params (TraceChannel :type "ETraceTypeQuery Enum" :default "TraceTypeQuery1"))
  (returns (HitActor :type "Actor Object Reference"))
  (bind _returnvalue (`SceneComponent.K2_GetComponentLocation` (`self.Camera`)))
  (bind _outhit (`KismetSystemLibrary.LineTraceSingle` :`Start` _returnvalue :`End` (+ _returnvalue (* (`KismetMathLibrary.GetForwardVector` (`SceneComponent.K2_GetComponentRotation` (`self.Camera`))) 1000.0)) :`TraceChannel` TraceChannel :`bTraceComplex` true :`DrawDebugType` "ForDuration"))
  (return (`.HitActor` (`GameplayStatics.BreakHitResult` _outhit))))

(fn `SetManagerVariable`
  (`|ExecutionSequence`
    (:`then_0`
      (bind _asbp_tomorrows_day_pc (cast `/Game/Blueprint/Global/BP_TomorrowsDay_PC` (`GameplayStatics.GetPlayerController` 0)))
      (set `self.Tomorrows Day PC` _asbp_tomorrows_day_pc))))

(fn `UserConstructionScript`
  (`self.ContraintViewAngle`))