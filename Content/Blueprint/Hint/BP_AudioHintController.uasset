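; Audio hint controller that plays puzzle hint sounds which are audible only while the camera's audio filter is active.
; After the scene manager initializes, it binds to HintManager filter and volume events and sets up the hint mesh.
; Filter changes mute or unmute the audio, showing the sound decal only under the audio filter during playback.
; ChangeAudioState selects a track from a map, handles play, pause or stop, then reapplies the current filter.
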(event `self.ReceiveBeginPlay`
  ;[1 1 1] Initialization Binding Event
  (bind _output_get (set `self.Scene Manager` (`/Game/Blueprint/Global/BFL_FunctionEverywhere.InitiateSceneManager`)))
  (add `/Game/Blueprint/Global/Manager/BP_SceneManager.OnInitiateManagerEvent` _output_get (delegate `Initialization_Event`)))

(event `Initialization_Event`
  ;[1 1 1] Initialization Binding Event
  (`|ExecutionSequence`
    (:`then_0`
      (`self.SetManagerVariable`))
    (:`then_1`
      (`self.Bind All Event`))
    (:`then_2`
      (`self.SetupHintMesh`))))

(event `BindActiveFilter`
  (add `/Game/Blueprint/Global/Manager/BP_HintManager.OnEnableFilterVisual` (`self.Hint Manager`) (delegate `ActiveFilter_Event`)))

(event `ActiveFilter_Event`
  (params (EActiveFilter :type "/Game/Data/Enumerator/Camera/ECameraFilter Enum" :default "NewEnumerator0"))
  (switch `/Game/Data/Enumerator/Camera/ECameraFilter` EActiveFilter
    (:`NewEnumerator0`
      (`self.SetVisibilityFIlter` false :!label _label)
      (`self.HandleVolume_Event` "NewEnumerator1"))
    (:`NewEnumerator1`
      (goto _label))
    (:`NewEnumerator2`
      (goto _label))
    (:`NewEnumerator3`
      (`self.SetVisibilityFIlter` (`AudioComponent.IsPlaying` (`self.Audio`)))
      (`self.HandleVolume_Event` "NewEnumerator2"))))

(event `ChangeAudioState`
  (params (`EAudio State` :type "/Game/Data/Enumerator/State/EAudioState Enum" :default "NewEnumerator0") (AudioPiste :type Integer))
  (`AudioComponent.SetSound` (`self.Audio`) (`BlueprintMapLibrary.Map_Find` (`self.AudioHint`) AudioPiste))
  (switch `/Game/Data/Enumerator/State/EAudioState` `EAudio State`
    (:`NewEnumerator1`
      (if (not (`AudioComponent.IsPlaying` (`self.Audio`)))
        (`AudioComponent.Play` (`self.Audio`) 0.0)
        (`self.Pause Audio` false)
        (`self.ActiveFilter_Event` (`/Game/Blueprint/Global/Manager/BP_CameraActorManager.ECurrentCameraFilter` (`/Game/Blueprint/Global/Manager/BP_SceneManager.CameraActorManager` (`self.Scene Manager`))) :!label _label_2)))
    (:`NewEnumerator2`
      (`self.Pause Audio` true)
      (goto _label_2))
    (:`NewEnumerator3`
      (`AudioComponent.Stop` (`self.Audio`))
      (goto _label_2))))

(event `Pause Audio`
  (params (bPause :type Boolean))
  (`AudioComponent.SetPaused` (`self.Audio`) bPause))

(event `BindHandleAudioVolume`
  (add `/Game/Blueprint/Global/Manager/BP_HintManager.OnToggleAudioVolume` (`self.Hint Manager`) (delegate `HandleVolume_Event`)))

(event `HandleVolume_Event`
  (params (`EAudio Volume` :type "/Game/Data/Enumerator/State/EAudioVolumeState Enum" :default "NewEnumerator0"))
  (switch `/Game/Data/Enumerator/State/EAudioVolumeState` `EAudio Volume`
    (:`NewEnumerator1`
      (`self.HandleAudioVolume` 0.0))
    (:`NewEnumerator2`
      (`self.HandleAudioVolume` 1.0))))

(fn `Bind All Event`
  (`self.BindHandleAudioVolume`)
  (`self.BindActiveFilter`))

(fn `HandleAudioVolume`
  (params (VolumeMultiplier :type "Float (single-precision)"))
  (`AudioComponent.SetVolumeMultiplier` (`self.Audio`) VolumeMultiplier))

(fn `SetVisibilityFIlter`
  (params (`Set Visibility` :type Boolean))
  (`SceneComponent.SetVisibility` (`self.Sound_Decal`) `Set Visibility` false))

(fn `UserConstructionScript`
  (`parent.UserConstructionScript`))