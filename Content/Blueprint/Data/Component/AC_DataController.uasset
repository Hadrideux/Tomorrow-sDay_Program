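; Data controller component that records and looks up found hint and citizen data for an investigation game.
; On BeginPlay it waits for the SceneManager's initiate event, then caches its DataManager and calls the event-binding functions.
; Helpers forward finds and lookups to the DataManager, list DataTable row names and do case-insensitive substring search.
; An analyse-break handler sets hint weight, but its InvestigationManager binding is disconnected.
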(event `self.ReceiveBeginPlay`
  ;[1 1 1] Initialization Binding Event
  (`self.BindInitiate`))

(event `BindInitiate`
  ;[1 1 1] Initialization Binding Event
  (bind _output_get (set `self.Scene Manager` (`/Game/Blueprint/Global/BFL_FunctionEverywhere.InitiateSceneManager`)))
  (add `/Game/Blueprint/Global/Manager/BP_SceneManager.OnInitiateManagerEvent` _output_get (delegate `Initiate Event`)))

(event `Initiate Event`
  ;[1 1 1] Initialization Binding Event
  (`|ExecutionSequence`
    (:`then_0`
      (`self.SetManagerVariable`))
    (:`then_1`
      (`self.BindAllEvent`))))

(event `BindAnalyseBreak`
  ;[1 1 1] Added Hint Information
)

(event `AnalyseBreak Event`
  (params (CurrentHint :type "/Game/Blueprint/Data/Component/AC_DataController Object Reference") (`Analyse Index` :type Integer))
  ;[1 1 1] Added Hint Information
  (if (== CurrentHint self)
    (set `self.CurrentAnalyseIndex` `Analyse Index`)
    (set `self.HintWeight` (`KismetMathLibrary.Conv_IntToDouble` `Analyse Index`))))

(fn `BindAllEvent`
  (`self.BindAnalyseBreak`)
  (`self.BindAnallyseInProgress`))

(fn `CitizenDataFind`
  (params (CitizenName :type Name) (CitizenDataFind :type "/Game/Data/Stucture/Citizen/SCitizenData Structure"))
  (`/Game/Blueprint/Global/Manager/BP_DataManager.AddCitizenData` (`self.DataManager`) CitizenName CitizenDataFind))

(fn `FindCitizenData`
  (params (CitizenName :type "Name (by ref)"))
  (returns (bIsCitizenFind :type Boolean))
  (return (`.ReturnValue` (`BlueprintMapLibrary.Map_Find` (`/Game/Blueprint/Global/Manager/BP_DataManager.CitizenDataAlreadyFind` (`self.DataManager`)) CitizenName))))

(fn `FindHintData`
  (params (HintName :type "Name (by ref)"))
  (returns (bIsHintFind :type Boolean))
  (return (`.ReturnValue` (`BlueprintMapLibrary.Map_Find` (`/Game/Blueprint/Global/Manager/BP_DataManager.HintDataAlreadyFind` (`self.DataManager`)) HintName))))

(fn `GetDataRowName`
  (params (DataTable :type "DataTable Object Reference"))
  (returns (CitizenRowNames :type "Array of Name"))
  (bind _outrownames (`DataTableFunctionLibrary.GetDataTableRowNames` DataTable))
  (return _outrownames))

(fn `HintDataFind`
  (params (HintName :type Name) (HintDataFind :type "/Game/Data/Stucture/Hint/SHintData Structure"))
  (`/Game/Blueprint/Global/Manager/BP_DataManager.AddHintData` (`self.DataManager`) HintName HintDataFind))

(fn `SearchExistInData`
  (params (RowData :type String) (Search :type Text))
  (returns (SearchContains :type Boolean))
  (bind _returnvalue (`KismetStringLibrary.ToLower` (`KismetTextLibrary.Conv_TextToString` Search)))
  (return (and (`KismetStringLibrary.Contains` (`KismetStringLibrary.ToLower` RowData) _returnvalue) (not (`KismetStringLibrary.IsEmpty` _returnvalue)))))

(fn `SetManagerVariable`
  (set `self.DataManager` (`/Game/Blueprint/Global/Manager/BP_SceneManager.DataManager` (`self.Scene Manager`))))