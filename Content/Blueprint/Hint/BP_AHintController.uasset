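; Hint actor that displays either a prop or a citizen according to its hint type (UV, thermal, audio or citizen).
; The construction script loads the mesh by HintName from DT_Hint or DT_Citizen and shows the matching static or skeletal component.
; Thermal and citizen hints also apply custom depth stencil settings for thermal rendering.
; A helper caches managers from SceneManager, while event binding and visibility filter functions are empty stubs.
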(event `SetupHintMesh`
  (bind (_hintdata _citizendata) (`self.SetupMesh`))
  (`|ExecutionSequence`
    (:`then_0`
      (`SkeletalMeshComponent.SetSkeletalMeshAsset` (`self.SkeletalMesh`) (`.SkeletalMesh_41_130E3F124CD095F1B7EDE8AA6B4EC006` (break `/Game/Data/Stucture/Citizen/SCitizenData` _citizendata))))
    (:`then_1`
      (`StaticMeshComponent.SetStaticMesh` (`self.Cube`) (`.StaticMesh_19_23E029DF4D593E8C0173BC83DFF0151B` (break `/Game/Data/Stucture/Hint/SHintData` _hintdata))))))

(fn `BindAllEvent`)

(fn `SetManagerVariable`
  (bind _scene_manager (`self.Scene Manager`))
  (set `self.Game State Manager` (`/Game/Blueprint/Global/Manager/BP_SceneManager.GameStateManager` _scene_manager))
  (set `self.Hint Manager` (`/Game/Blueprint/Global/Manager/BP_SceneManager.HintManager` _scene_manager))
  (set `self.Sequencer Manager` (`/Game/Blueprint/Global/Manager/BP_SceneManager.SequencerManager` _scene_manager))
  (set `self.Camera Actor Manager` (`/Game/Blueprint/Global/Manager/BP_SceneManager.CameraActorManager` _scene_manager))
  (set `self.Data Manager` (`/Game/Blueprint/Global/Manager/BP_SceneManager.DataManager` _scene_manager)))

(fn `SetupMesh`
  (returns (HintData :type "/Game/Data/Stucture/Hint/SHintData Structure") (CitizenData :type "/Game/Data/Stucture/Citizen/SCitizenData Structure"))
  (bind _hintname (`self.HintName`))
  (switch `/Game/Data/Enumerator/Data/EHintType` (`self.EHintType`)
    (:`NewEnumerator1`
      _)
    (:`NewEnumerator2`
      _)
    (:`NewEnumerator3`
      _)
    (:`NewEnumerator4`
      (bind _returnvalue (`|GetDataTableRow` "/Game/Data/DT_Citizen.DT_Citizen" _hintname)
        (:`then`
          (return (struct) _returnvalue)))))
  (bind _returnvalue_2 (`|GetDataTableRow` "/Game/Data/DT_Hint.DT_Hint" _hintname)
    (:`then`
      (return _returnvalue_2))))

(fn `SetVisibilityFIlter`
  (params (`Set Visibility` :type Boolean)))

(fn `UserConstructionScript`
  (bind _skeletalmesh (`self.SkeletalMesh`))
  (bind _cube (`self.Cube`))
  (`|ExecutionSequence`
    (:`then_0`
      (`self.SetupHintMesh`))
    (:`then_1`
      (switch `/Game/Data/Enumerator/Data/EHintType` (`self.EHintType`)
        (:`NewEnumerator1`
          (`SceneComponent.SetVisibility` (`self.Cube`) true false :!label _label)
          (`SceneComponent.SetVisibility` (`self.SkeletalMesh`) false false))
        (:`NewEnumerator2`
          (`PrimitiveComponent.SetRenderCustomDepth` _cube (`self.ThermalRender`))
          (`PrimitiveComponent.SetCustomDepthStencilValue` _cube (`self.ThermalStencilValue`))
          (goto _label))
        (:`NewEnumerator3`
          (goto _label))
        (:`NewEnumerator4`
          (`SceneComponent.SetVisibility` (`self.SkeletalMesh`) true false)
          (`PrimitiveComponent.SetRenderCustomDepth` _skeletalmesh (`self.ThermalRender`))
          (`PrimitiveComponent.SetCustomDepthStencilValue` _skeletalmesh (`self.ThermalStencilValue`))
          (`SceneComponent.SetVisibility` (`self.Cube`) false false))))))