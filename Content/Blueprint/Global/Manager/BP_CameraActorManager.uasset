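; Camera manager that shows and hides the camera interface and tracks the active camera filter.
; Once the SceneManager signals initiation, it caches the UI and Sequencer managers, binds filter changes and applies a default filter.
; It also sets the interface timecode's maximum from the current Level Sequence's end frame.
; Filter changes store the filter and post-process index, then tell the HintManager to update filter visuals.
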(event `self.ReceiveBeginPlay`
  ;[1 1 1] Initialization
  (bind _output_get (set `self.Scene Manager` (`/Game/Blueprint/Global/BFL_FunctionEverywhere.InitiateSceneManager`)))
  (add `/Game/Blueprint/Global/Manager/BP_SceneManager.OnInitiateManagerEvent` _output_get (delegate `Initiate_Event`)))

(event `Initiate_Event`
  ;[1 1 1] Initialization
  (`|ExecutionSequence`
    (:`then_0`
      (`self.SetManagerVariable`))
    (:`then_1`
      (`self.BindEvent`))
    (:`then_2`
      (`self.SetMaxTimecode`)
      (`self.OnChangeFilter` "NewEnumerator0"))))

(event `SetMaxTimecode`
  (set `Slider.MaxValue` (`KismetMathLibrary.Conv_IntToDouble` (break `FrameNumber` (break `QualifiedFrameTime` (`MovieSceneSequencePlayer.GetEndTime` (`/Game/Blueprint/Global/Manager/BP_SequencerManager.Current Level Sequence` (`self.Sequencer Manager`)))))) (`/Game/Widget/Camera/WBP_CameraInterface.Timecode` (`/Game/Blueprint/Global/Manager/BP_UIManager.CameraInterface` (`self.UIManager`)))))

(event `BindCameraFilter`
  (add `self.OnChangeFilter` (delegate `ChangeFilter_Event`)))

(event `ChangeFilter_Event` :!signature `self.OnChangeFilter`
  (params (ESelectedFilter :type "/Game/Data/Enumerator/Camera/ECameraFilter Enum" :default "NewEnumerator0") (PostProcessIndex :type Integer))
  (set `self.ECurrentCameraFilter` ESelectedFilter)
  (set `self.Current PostProcess Index` PostProcessIndex)
  (`|ExecutionSequence`
    (:`then_0`
      (`/Game/Blueprint/Global/Manager/BP_HintManager.OnEnableFilterVisual` (`/Game/Blueprint/Global/Manager/BP_SceneManager.HintManager` (`self.Scene Manager`)) (`self.ECurrentCameraFilter`)))))

(fn `BindEvent`
  (`self.BindCameraFilter`))

(fn `DisplayCameraInterface`
  (bind _uimanager (`self.UIManager`))
  (`/Game/Blueprint/Global/Manager/BP_UIManager.DisplayWidget` _uimanager true (`/Game/Blueprint/Global/Manager/BP_UIManager.CameraInterface` _uimanager)))

(fn `RemoveCameraInterface`
  (bind _uimanager (`self.UIManager`))
  (`/Game/Blueprint/Global/Manager/BP_UIManager.RemoveWidget` _uimanager (`/Game/Blueprint/Global/Manager/BP_UIManager.CameraInterface` _uimanager)))

(fn `SetManagerVariable`
  (bind _scene_manager (`self.Scene Manager`))
  (set `self.UIManager` (`/Game/Blueprint/Global/Manager/BP_SceneManager.UIManager` _scene_manager))
  (set `self.Sequencer Manager` (`/Game/Blueprint/Global/Manager/BP_SceneManager.SequencerManager` _scene_manager)))

(fn `UserConstructionScript`)