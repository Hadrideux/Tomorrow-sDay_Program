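; Camera controller actor that moves between preset camera positions and lets the player select hints through the camera view.
; After SceneManager initializes, it caches managers, binds position-change and interact events, and snaps to the first position.
; Interaction sphere-traces along the camera's forward vector, despite the mouse-based name, and passes any hit hint controller to CameraActorManager.
; A filter handler drives ACCameraFilter post-process visuals, though BindAllEvent never binds it.
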(event `self.ReceiveBeginPlay`
  ;[1 1 1] Initialization Binding Event
  (bind _output_get (set `self.Scene Manager` (`/Game/Blueprint/Global/BFL_FunctionEverywhere.InitiateSceneManager`)))
  (add `/Game/Blueprint/Global/Manager/BP_SceneManager.OnInitiateManagerEvent` _output_get (delegate `Initialization_Event`)))

(event `Initialization_Event`
  ;[1 1 1] Initialization Binding Event
  (`|ExecutionSequence`
    (:`then_0`
      (`self.SetManagerVariable`))
    (:`then_1`
      (`self.Bind All Event`))
    (:`then_2`
      (`self.HandleCameraLocation` 0))))

(event `DisplayCameraWidget`
  ;[1 1 1] Display/Remove Widget
  (`/Game/Blueprint/Global/Manager/BP_CameraActorManager.DisplayCameraInterface` (`self.CameraActor Manager`)))

(event `RemoveCameraWidget`
  ;[1 1 1] Display/Remove Widget
  (`/Game/Blueprint/Global/Manager/BP_CameraActorManager.RemoveCameraInterface` (`self.CameraActor Manager`)))

(event `BindFocusElement`
  (add `/Game/Blueprint/Global/BP_TomorrowsDay_PC.OnPlayerInteract` (`self.Tomorrows Day PC`) (delegate `FocusCamera_Event`)))

(event `FocusCamera_Event`
  (bind _hitactor (`self.Mouse Position to World Location`))
  (bind _asbp_ahint_controller (cast `/Game/Blueprint/Hint/BP_AHintController` _hitactor))
  (`/Game/Blueprint/Global/Manager/BP_CameraActorManager.OnHintSelect` (`self.CameraActor Manager`) _asbp_ahint_controller))

(event `BindChangeCamera`
  ;[1 0.1098 0.0902] Change Camera Position
  (add `/Game/Blueprint/Global/Manager/BP_CameraActorManager.OnChangeCameraPositon` (`self.CameraActor Manager`) (delegate `ChangeCameraPosition`)))

(event `BindFilterEvent`
  ;[0.102 0.2196 1] Filter Change Event
  (add `/Game/Blueprint/Global/Manager/BP_CameraActorManager.OnChangeFilter` (`self.CameraActor Manager`) (delegate `OnChangeFilter_Event`)))

(event `ChangeCameraPosition`
  (params (CameraPositionIndex :type Integer))
  ;[1 0.1098 0.0902] Change Camera Position
  (`self.HandleCameraLocation` CameraPositionIndex))

(event `OnChangeFilter_Event`
  (params (ESelectedFilter :type "/Game/Data/Enumerator/Camera/ECameraFilter Enum" :default "NewEnumerator0") (PostProcessIndex :type Integer))
  ;[0.102 0.2196 1] Filter Change Event
  (`/Game/Blueprint/Camera/Component/AC_CameraFilter.HandleFilterVisual` (`self.AC_CameraFilter`) ESelectedFilter PostProcessIndex))

(fn `Bind All Event`
  (`|ExecutionSequence`
    (:`then_0`
      (`self.BindChangeCamera`)
      (`self.BindChangeCamera`))
    (:`then_1`
      (`self.BindFocusElement`))))

(fn `HandleCameraLocation`
  (params (Position :type Integer))
  (bind _output (`|GetArrayItem` (`/Game/Blueprint/Global/Manager/BP_CameraActorManager.CameraPosition` (`self.CameraActor Manager`)) Position))
  (`/Engine/EditorBlueprintResources/StandardMacros.IsValid` _output
    (:`Is Valid`
      (`self.K2_SetActorTransform` self (`self.GetTransform` _output) true false))))

(fn `Mouse Position to World Location`
  (returns (HitActor :type "Actor Object Reference"))
  (bind _returnvalue (* (`KismetMathLibrary.GetForwardVector` (`SceneComponent.K2_GetComponentRotation` (`self.Camera`))) 1000.0))
  (bind _outhit (`KismetSystemLibrary.SphereTraceSingle` :`Start` (+ (`SceneComponent.K2_GetComponentLocation` (`self.Camera`)) _returnvalue) :`End` _returnvalue :`Radius` (`self.Radius Spehre Trace`) :`TraceChannel` (`self.Trace Channel`) :`DrawDebugType` (`self.Draw Debug Type`)))
  (return (`.HitActor` (`GameplayStatics.BreakHitResult` _outhit))))

(fn `SequenceControl`
  (params (SequencerState :type "/Game/Data/Enumerator/State/ESequencerState Enum" :default "NewEnumerator0"))
  (`/Game/Blueprint/Global/Manager/BP_SequencerManager.OnSequenceStateChange` (`self.Sequencer Manager`) SequencerState))

(fn `SetManagerVariable`
  (bind _scene_manager (`self.Scene Manager`))
  (`|ExecutionSequence`
    (:`then_0`
      (set `self.Tomorrows Day PC` (cast `/Game/Blueprint/Global/BP_TomorrowsDay_PC` (`GameplayStatics.GetPlayerController` 0) :!pure true)))
    (:`then_1`
      (set `self.UIManager` (`/Game/Blueprint/Global/Manager/BP_SceneManager.UIManager` _scene_manager))
      (set `self.CameraActor Manager` (`/Game/Blueprint/Global/Manager/BP_SceneManager.CameraActorManager` _scene_manager)))
    (:`then_2`
      (set `self.Sequencer Manager` (`/Game/Blueprint/Global/Manager/BP_SceneManager.SequencerManager` (`self.Scene Manager`))))
    (:`then_3`
      (set `self.Hint Manager` (`/Game/Blueprint/Global/Manager/BP_SceneManager.HintManager` (`self.Scene Manager`))))))

(fn `UserConstructionScript`
  (bind _scenecapturecomponent2d (`self.SceneCaptureComponent2D`))
  (`/Engine/EditorBlueprintResources/StandardMacros.IsValid` (`SceneCaptureComponent2D.TextureTarget` _scenecapturecomponent2d)
    (:`Is Valid`
      (set `SceneCaptureComponent2D.TextureTarget` "/Game/Asset/Texture/CameraView/RT_CameraView.RT_CameraView" _scenecapturecomponent2d))))