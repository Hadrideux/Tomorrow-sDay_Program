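; UI manager that pre-creates the game's menu, hub, Regis, camera and mission widgets on BeginPlay and holds references to them.
; Helper functions add or remove widgets from the viewport and toggle input mode and mouse cursor.
; Once SceneManager signals initialization, it caches CameraActorManager and binds to its filter change event.
; The audio filter shows the camera interface's audio analysis panel, while other filters show citizen and hint panels.
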(event `self.ReceiveBeginPlay`
  (`self.BindInitiate`))

(event `BindInitiate`
  (bind _output_get (set `self.Scene Manager` (`/Game/Blueprint/Global/BFL_FunctionEverywhere.InitiateSceneManager`)))
  (add `/Game/Blueprint/Global/Manager/BP_SceneManager.OnInitiateManagerEvent` _output_get (delegate `InitiateEvent`))
  (`self.CreateAllWidgets`))

(event `InitiateEvent`
  (`|ExecutionSequence`
    (:`then_0`
      (`self.SetManagerViariable`))
    (:`then_1`
      (`self.BindAllEvent`))))

(event `BindChangeFilter`
  (add `/Game/Blueprint/Global/Manager/BP_CameraActorManager.OnChangeFilter` (`self.Camera Actor Manager`) (delegate `EnableAnalyseWidget`)))

(event `EnableAnalyseWidget`
  (params (ESelectedFilter :type "/Game/Data/Enumerator/Camera/ECameraFilter Enum" :default "NewEnumerator0") (PostProcessIndex :type Integer))
  (bind _camerainterface (`self.CameraInterface`))
  (switch `/Game/Data/Enumerator/Camera/ECameraFilter` ESelectedFilter
    (:`NewEnumerator0`
      (`/Game/Widget/Camera/WBP_CameraInterface.SetAnalysePanel` _camerainterface false true true :!label _label))
    (:`NewEnumerator1`
      (goto _label))
    (:`NewEnumerator2`
      (goto _label))
    (:`NewEnumerator3`
      (`/Game/Widget/Camera/WBP_CameraInterface.SetAnalysePanel` _camerainterface true false false))))

(fn `BindAllEvent`
  (`self.BindChangeFilter`))

(fn `CreateAllWidgets`
  (`|ExecutionSequence`
    (:`then_0`
      ;[0 0.8332 1] Menu
      (bind _returnvalue (`|CreateWidget` "/Game/Widget/Menu/WBP_MainMenu.WBP_MainMenu_C"))
      (set `self.MainMenu` _returnvalue)
      (bind _returnvalue_2 (`|CreateWidget` "/Game/Widget/Menu/WBP_SettingsMenu.WBP_SettingsMenu_C"))
      (set `self.SettingsMenu` _returnvalue_2)
      (bind _returnvalue_3 (`|CreateWidget` "/Game/Widget/Menu/WBP_CreditsMenu.WBP_CreditsMenu_C"))
      (set `self.CreditsMenu` _returnvalue_3)
      (bind _returnvalue_4 (`|CreateWidget` "/Game/Widget/Menu/WBP_PauseMenu.WBP_PauseMenu_C"))
      (set `self.PauseMenu` _returnvalue_4))
    (:`then_1`
      ;[0 0.8332 1] Hub Screen
      (bind _returnvalue_5 (`|CreateWidget` "/Game/Widget/HUBScreen/WBP_HUBScreen.WBP_HUBScreen_C"))
      (set `self.HubScreen` _returnvalue_5)
      (bind _returnvalue_6 (`|CreateWidget` "/Game/Widget/HUBScreen/MapDallas/WBP_DallasMap.WBP_DallasMap_C"))
      (set `self.DallasMap` _returnvalue_6)
      (bind _returnvalue_7 (`|CreateWidget` "/Game/Widget/HUBScreen/InformationsCenter/WBP_DataCenter.WBP_DataCenter_C"))
      (set `self.DataCenter` _returnvalue_7)
      (bind _returnvalue_8 (`|CreateWidget` "/Game/Widget/HUBScreen/AnalysisReport/WBP_AnalysisReport.WBP_AnalysisReport_C"))
      (set `self.AnalysisReport` _returnvalue_8))
    (:`then_2`
      ;[0 0.8332 1] Regis Screen
      (bind _returnvalue_9 (`|CreateWidget` "/Game/Widget/RegisScreen/WBP_RegisInterface.WBP_RegisInterface_C"))
      (set `self.RegisScreen` _returnvalue_9)
      (bind _returnvalue_10 (`|CreateWidget` "/Game/Widget/Camera/WBP_CameraInterface.WBP_CameraInterface_C"))
      (set `self.CameraInterface` _returnvalue_10)
      (bind _returnvalue_11 (`|CreateWidget` "/Game/Widget/Camera/Analyse/WBP_HintAnalyse.WBP_HintAnalyse_C"))
      (set `self.HintAnalysis` _returnvalue_11))
    (:`then_3`
      ;[0 0.8332 1] Miscellaneous
      (bind _returnvalue_12 (`|CreateWidget` "/Game/Widget/CorkBoard/WBP_MissionOrder.WBP_MissionOrder_C"))
      (set `self.MissionOrder` _returnvalue_12)
      (bind _returnvalue_13 (`|CreateWidget` "/Game/Widget/CorkBoard/WBP_CorkBoardHUD.WBP_CorkBoardHUD_C"))
      (set `self.CorkboardHUD` _returnvalue_13))))

(fn `DisplayWidget`
  (params (isUIMode :type Boolean) (ShowWidget :type "UserWidget Object Reference"))
  (`UserWidget.AddToViewport` ShowWidget 0)
  (`self.InitializeWidget` isUIMode))

(fn `InitializeWidget`
  (params (Condition :type Boolean))
  (bind _returnvalue (`GameplayStatics.GetPlayerController` 0))
  (bind _returnvalue_2 (`GameplayStatics.GetPlayerController` 0))
  (if Condition
    (`WidgetBlueprintLibrary.SetInputMode_GameAndUIEx` _returnvalue (`self.CurrentWidget`))
    (set `PlayerController.bShowMouseCursor` true _returnvalue)
    (else
      (`WidgetBlueprintLibrary.SetInputMode_GameOnly` _returnvalue_2)
      (set `PlayerController.bShowMouseCursor` false _returnvalue_2))))

(fn `RemoveWidget`
  (params (RemoveWidget :type "UserWidget Object Reference"))
  (if (`Widget.IsInViewport` RemoveWidget)
    (`Widget.RemoveFromParent` RemoveWidget)))

(fn `SetManagerViariable`
  (set `self.Camera Actor Manager` (`/Game/Blueprint/Global/Manager/BP_SceneManager.CameraActorManager` (`self.Scene Manager`))))

(fn `UserConstructionScript`)