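; BP_HintManager is a manager Blueprint that keeps track of the currently selected hint.
; On BeginPlay it obtains the SceneManager and waits for its manager-initiation event before binding anything.
; It then subscribes to the CameraActorManager's hint-select event and stores each received selection as CurrentHintSelected, with no further handling in this graph.
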(event `self.ReceiveBeginPlay`
  (`self.Initiate`))

(event `Initiate`
  (bind _output_get (set `self.Scene Manager` (`/Game/Blueprint/Global/BFL_FunctionEverywhere.InitiateSceneManager`)))
  (add `/Game/Blueprint/Global/Manager/BP_SceneManager.OnInitiateManagerEvent` _output_get (delegate `Initialization_Event`)))

(event `Initialization_Event`
  (`|ExecutionSequence`
    (:`then_1`
      (`self.BindHintSelect`))))

(event `BindHintSelect`
  (add `/Game/Blueprint/Global/Manager/BP_CameraActorManager.OnHintSelect` (`/Game/Blueprint/Global/Manager/BP_SceneManager.CameraActorManager` (`self.Scene Manager`)) (delegate `HintSelect_Event`)))

(event `HintSelect_Event`
  (params (HintSelect :type "/Game/Blueprint/Hint/BP_AHintController Object Reference"))
  (set `self.CurrentHintSelected` HintSelect))

(fn `UserConstructionScript`)