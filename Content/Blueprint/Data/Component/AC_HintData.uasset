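; Hint data component that answers the DataManager's data requests for UV, thermal and audio hints, bound through a camera-named event.
; It casts the hint by type, then either resends the DataManager's already-found citizen and hint data or searches a hint DataTable by name.
; The search compares only each row's unfiltered text fields and passes a matching hint name to CitizenDataFind, relying on parent-class helpers for row listing, matching and lookup.
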(event `BindRequestDataFromCamera`
  (add `/Game/Blueprint/Global/Manager/BP_DataManager.OnRequestData` (`self.DataManager`) (delegate `RequestData_Event`)))

(event `RequestData_Event`
  (params (`BP Hint` :type "/Game/Blueprint/Hint/BP_AHintController Object Reference") (SearchEntryComitted :type Text))
  (bind _datamanager (`self.DataManager`))
  (bind _output_get (set `self.BP Hint` `BP Hint`))
  (if (not (`KismetSystemLibrary.IsValid` _output_get))
    (switch `/Game/Data/Enumerator/Data/EHintType` (`/Game/Blueprint/Hint/BP_AHintController.EHintType` _output_get)
      (:`NewEnumerator1`
        (bind _asbp_uvhint_controller (cast `/Game/Blueprint/Hint/BP_UVHintController` (`self.BP Hint`)))
        (if (`self.FindHintData` (`/Game/Blueprint/Hint/BP_AHintController.HintName` _asbp_uvhint_controller))
          (`/Game/Blueprint/Global/Manager/BP_DataManager.OnSendData` _datamanager (`/Game/Blueprint/Global/Manager/BP_DataManager.CitizenDataAlreadyFind` _datamanager) (`/Game/Blueprint/Global/Manager/BP_DataManager.HintDataAlreadyFind` _datamanager) "None" :!label _label)
          (else
            (`self.SearchData` (`/Game/Blueprint/Hint/BP_AHintController.HintName` (`self.BP Hint`))))))
      (:`NewEnumerator2`
        (bind _asbp_thermal_hint_controller (cast `/Game/Blueprint/Hint/BP_ThermalHintController` (`self.BP Hint`)))
        (if (`self.FindHintData` (`/Game/Blueprint/Hint/BP_AHintController.HintName` _asbp_thermal_hint_controller))
          (goto _label)
          (else
            (`self.SearchData` (`/Game/Blueprint/Hint/BP_AHintController.HintName` (`self.BP Hint`))))))
      (:`NewEnumerator3`
        (bind _asbp_audio_hint_controller (cast `/Game/Blueprint/Hint/BP_AudioHintController` (`self.BP Hint`)))
        (if (`self.FindHintData` (`/Game/Blueprint/Hint/BP_AHintController.HintName` _asbp_audio_hint_controller))
          (goto _label)
          (else
            (`self.SearchData` (`/Game/Blueprint/Hint/BP_AHintController.HintName` (`self.BP Hint`)))))))))

(event `SearchData`
  (params (HintName :type Name))
  (bind _value (`BlueprintMapLibrary.Map_Find` (`/Game/Blueprint/Global/Manager/BP_DataManager.AllDataTable` (`self.DataManager`)) "NewEnumerator2"))
  (bind _citizenrownames (`self.GetDataRowName` _value))
  (for _array_element _citizenrownames :!label _label
    (bind _array (`self.Get Data Hint` _value _array_element))
    (for _array_element_2 _array
      (bind _searchcontains (`self.SearchExistInData` _array_element_2 (`KismetTextLibrary.Conv_NameToText` HintName)))
      (if _searchcontains
        (`|ExecutionSequence`
          (:`then_0`
            (goto _label :!via `Break`))
          (:`then_1`
            (`self.CitizenDataFind` HintName)))))))

(fn `CitizenDataFind`
  (params (CitizenName :type Name) (CitizenDataFind :type "/Game/Data/Stucture/Citizen/SCitizenData Structure"))
  (`parent.CitizenDataFind` CitizenName CitizenDataFind))

(fn `Get Data Hint`
  (params (`Data Table` :type "DataTable Object Reference") (`Row Name` :type Name))
  (returns (Array :type "Array of String") (`Out Row` :type "/Game/Data/Stucture/Hint/SHintData Structure"))
  (bind _returnvalue (`|GetDataTableRow` `Data Table` `Row Name`)
    (:`then`
      (bind (_name _description _manufacturer _datepurchase _dimension _weight) (break `/Game/Data/Stucture/Hint/SHintNoFilterData` (`.NoFilter_9_A007747B464D11C439FB1C9F72A89AF7` (break `/Game/Data/Stucture/Hint/SHintData` _returnvalue))))
      (return (`|MakeArray` (`KismetTextLibrary.Conv_TextToString` _name) (`KismetTextLibrary.Conv_TextToString` _description) (`KismetTextLibrary.Conv_TextToString` _manufacturer) (`KismetTextLibrary.Conv_TextToString` _datepurchase) (`KismetStringLibrary.Conv_VectorToString` _dimension) (`KismetStringLibrary.Conv_DoubleToString` _weight) "" "") _returnvalue))))

(fn `GetDataRowName`
  (params (DataTable :type "DataTable Object Reference"))
  (returns (CitizenRowNames :type "Array of Name"))
  (bind _citizenrownames (`parent.GetDataRowName` DataTable))
  (return _citizenrownames))

(fn `SearchDartaFromDataCenter`
  (params (`Search Entry Committed` :type Text)))

(fn `SearchExistInData`
  (params (RowData :type String) (Search :type Text))
  (returns (SearchContains :type Boolean))
  (bind _searchcontains (`parent.SearchExistInData` RowData Search))
  (return _searchcontains))