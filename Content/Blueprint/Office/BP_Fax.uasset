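; Office fax actor that signals the state of investigation hint analysis through a colored point light.
; On BeginPlay it waits for the SceneManager singleton's init event, caches the InvestigationManager, binds analysis completion and shows green for printing available.
; Handlers also define orange for incoming and hidden for none, but the analysis-request and print bindings are never run here.
; StartNewInvestigation triggers a new investigation and clears the light.
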(event `BindInit`
  ;[1 1 1] Initialization Binding Event
  (bind _output_get (set `self.Scene Manager` (cast `/Game/Blueprint/Global/Manager/BP_SceneManager` (`/Game/Blueprint/Global/BFL_FunctionEverywhere.GetSingletonInstance` "/Game/Blueprint/Global/Manager/BP_SceneManager.BP_SceneManager_C") :!pure true)))
  (add `/Game/Blueprint/Global/Manager/BP_SceneManager.OnInitiateManagerEvent` _output_get (delegate `BindInitEvent`)))

(event `BindInitEvent`
  ;[1 1 1] Initialization Binding Event
  (`|ExecutionSequence`
    (:`then_0`
      (`self.SetManagerVariable` (`self.Scene Manager`)))
    (:`then_1`
      (`self.BindAllEvent`)
      (`self.PrintingAvailable`))))

(event `self.ReceiveBeginPlay`
  ;[1 1 1] Initialization Binding Event
  (`self.BindInit`))

(event `StartNewInvestigation`
  ;[1 1 1] Start Investigation
  (`/Game/Blueprint/Global/Manager/BP_InvestigationManager.OnNewInvestigation` (`self.Investigation Manager`))
  (`self.NoPrinting`))

(event `BindPrintAnalyse`
  ;[1 1 1] Data Avaible from Hint Analyse
  (add `/Game/Blueprint/Global/Manager/BP_InvestigationManager.OnPrintAnalyse` (`self.Investigation Manager`) (delegate `PrintAnalyse_Event`)))

(event `BindNewHint`
  ;[1 1 1] Data Avaible from Hint Analyse
  (add `/Game/Blueprint/Global/Manager/BP_InvestigationManager.OnAnalyseComplete` (`self.Investigation Manager`) (delegate `AnalyseComplete_Event`)))

(event `BindAnalyseInProgress`
  ;[1 1 1] Data Avaible from Hint Analyse
)

(event `AnalyseComplete_Event`
  (params (CurrentHint :type "/Game/Blueprint/Data/Component/AC_DataController Object Reference") (`Analyse Index` :type Integer))
  ;[1 1 1] Data Avaible from Hint Analyse
  (`self.PrintingAvailable`))

(event `AnalyseRequest_Event`
  (params (`Hint For Analyse` :type "Object Object Reference") (AnalyseState :type "/Game/Data/Enumerator/State/EAnalysisState Enum" :default "NewEnumerator0"))
  ;[1 1 1] Data Avaible from Hint Analyse
  (switch `/Game/Data/Enumerator/State/EAnalysisState` AnalyseState
    (:`NewEnumerator1`
      (`self.PrintingIncoming`))
    (:`NewEnumerator2`
      (`self.NoPrinting`))))

(event `PrintAnalyse_Event`
  ;[1 1 1] Data Avaible from Hint Analyse
  (`self.NoPrinting`))

(event `PrintingAvailable`
  ;[1 1 1] Light FeedBack Data
  (`self.SetDataLight` (`self.PointLight`) (struct :`R` 0.11972 :`G` 0.786458 :`B` 0.086654 :`A` 1.0) true))

(event `PrintingIncoming`
  ;[1 1 1] Light FeedBack Data
  (`self.SetDataLight` (`self.PointLight`) (struct :`R` 0.848958 :`G` 0.361949 :`B` 0.05306 :`A` 1.0) true))

(event `NoPrinting`
  ;[1 1 1] Light FeedBack Data
  (`self.SetDataLight` (`self.PointLight`) (struct :`R` 1.0 :`G` 1.0 :`B` 1.0 :`A` 1.0)))

(fn `BindAllEvent`
  (`self.BindNewHint`)
  (`self.BindAnalyseInProgress`))

(fn `GetAnalyse`)

(fn `SetDataLight`
  (params (Light :type "PointLightComponent Object Reference") (LightColor :type "LinearColor Structure") (bIsVisibility :type Boolean))
  (`LightComponent.SetLightColor` Light LightColor true)
  (`SceneComponent.SetVisibility` Light bIsVisibility false))

(fn `SetManagerVariable`
  (params (SceneManager :type "/Game/Blueprint/Global/Manager/BP_SceneManager Object Reference"))
  (set `self.Investigation Manager` (`/Game/Blueprint/Global/Manager/BP_SceneManager.InvestigationManager` SceneManager)))

(fn `UserConstructionScript`
  (`SceneComponent.SetVisibility` (`self.PointLight`) true false))