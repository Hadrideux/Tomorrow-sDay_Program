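; Player controller for an office scene that moves the player between the character, desk screens and a camera actor.
; Once the scene manager initiates, it caches managers, adds Enhanced Input contexts and binds to the pawn-change event.
; Pawns come from the ComputerManager's desk element map, possessed after short delays, with view blends for screens.
; Possess and unpossess handlers toggle HUB or camera widgets and cursor, while look and interact input is rebroadcast.
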(event `self.ReceiveBeginPlay`
  ;[1 1 1] Initiate
  (`self.BindInitiate`))

(event `ShowMouseCursor`
  (params (`Show Mouse Cursor` :type Boolean))
  ;[1 1 1] Showing Mouse Cursor
  (set `self.bShowMouseCursor` `Show Mouse Cursor`))

(event `BindInitiate`
  ;[1 1 1] Initiate
  (bind _output_get (set `self.Scene Manager` (`/Game/Blueprint/Global/BFL_FunctionEverywhere.InitiateSceneManager`)))
  (add `/Game/Blueprint/Global/Manager/BP_SceneManager.OnInitiateManagerEvent` _output_get (delegate `Initiate`)))

(event `Initiate`
  ;[1 1 1] Initiate
  (`|ExecutionSequence`
    (:`then_0`
      (`self.Input Mapping Initiate`)
      (`self.SetManagerVariable`))
    (:`then_1`
      (`self.BindAllEvent`))))

(event `EnhancedInput|/Game/Blueprint/Character/Input/Action/Game/Player/IA_LookAt`
  (params (ActionValue :type "Vector2D Structure") (ElapsedSeconds :type "Float (double-precision)") (TriggeredSeconds :type "Float (double-precision)") (InputAction :type "InputAction Object Reference" :default "/Game/Blueprint/Character/Input/Action/Game/Player/IA_LookAt.IA_LookAt"))
  ;[0.05098 0.6118 1] LookAt
  (:`Triggered`
    (`self.OnLookAt` ActionValue)))

(event `EnhancedInput|/Game/Blueprint/Character/Input/Action/Game/Player/IA_Interact`
  (params (ActionValue :type Boolean) (ElapsedSeconds :type "Float (double-precision)") (TriggeredSeconds :type "Float (double-precision)") (InputAction :type "InputAction Object Reference" :default "/Game/Blueprint/Character/Input/Action/Game/Player/IA_Interact.IA_Interact"))
  ;[0.05098 0.6118 1] Interact Input
  (:`Started`
    (`self.OnPlayerInteract`)))

(event `PlayerCharacterInputMapping`
  ;[0.05098 0.6118 1] Setup Input Mapping
  (`self.AddMappingContext` "/Game/Blueprint/Character/Input/IMC_Default.IMC_Default"))

(event `BindChangePosses`
  ;[1 1 1] hangement de pawn/ Ajouté condition d'ou on viens pour aller la ou on veux
  ;;[1 1 1] Comment
  ;;;[1 1 1] Event Changing PawnPossess
  (add `self.OnChangePossesPawn` (delegate `LeaveScreen_Event`)))

(event `LeaveScreen_Event` :!signature `self.OnChangePossesPawn`
  (params (OfficeElement :type "/Game/Data/Enumerator/Desk/EOfficeElement Enum" :default "NewEnumerator0"))
  ;[1 1 1] hangement de pawn/ Ajouté condition d'ou on viens pour aller la ou on veux
  ;;[1 1 1] Comment
  ;;;[1 1 1] Event Changing PawnPossess
  (set `self.Current Office Element` OfficeElement)
  (switch `/Game/Data/Enumerator/Desk/EOfficeElement` OfficeElement
    (:`NewEnumerator1`
      (`self.PossessNewPawn` OfficeElement)
      (`self.PossessCameraActor`))
    (:`NewEnumerator2`
      (if (`|EnumInequality` (`self.Current Office Element`) "NewEnumerator1")
        (`self.PossessNewPawn` OfficeElement)
        (else
          (`self.Possess` (`BlueprintMapLibrary.Map_Find` (`/Game/Blueprint/Global/Manager/BP_ComputerManager.DeskElement` (`self.Computer Manager`)) "NewEnumerator2"))
          (`self.PossessNewPawn` OfficeElement))))
    (:`NewEnumerator3`
      (`self.PossessCameraActor`))
    (:`NewEnumerator4`
      (`self.PossessPlayerCharacter`))))

(event `PossessCameraActor`
  (bind _value (`BlueprintMapLibrary.Map_Find` (`/Game/Blueprint/Global/Manager/BP_ComputerManager.DeskElement` (`self.Computer Manager`)) "NewEnumerator3"))
  ;[1 1 1] hangement de pawn/ Ajouté condition d'ou on viens pour aller la ou on veux
  ;;[1 1 1] Comment
  ;;;[1 1 1] Possess CameraActor/PlayerCharacter
  (`KismetSystemLibrary.Delay` 0.5)
  (`self.Possess` _value)
  (bind _asbp_camera_controller (cast `/Game/Blueprint/Camera/BP_CameraController` _value))
  (`/Game/Blueprint/Camera/BP_CameraController.DisplayCameraWidget` _asbp_camera_controller)
  (`self.ShowMouseCursor` true))

(event `PossessNewPawn`
  (params (Key :type "/Game/Data/Enumerator/Desk/EOfficeElement Enum (by ref)"))
  (bind _value (`self.FindOfficeElement` Key))
  ;[1 1 1] hangement de pawn/ Ajouté condition d'ou on viens pour aller la ou on veux
  ;;[1 1 1] Comment
  ;;;[1 1 1] Possess Desk Element
  (`self.SetPossessTransistion` _value)
  (`KismetSystemLibrary.Delay` 0.5)
  (`self.Possess` _value))

(event `PossessPlayerCharacter`
  ;[1 1 1] hangement de pawn/ Ajouté condition d'ou on viens pour aller la ou on veux
  ;;[1 1 1] Comment
  ;;;[1 1 1] Possess CameraActor/PlayerCharacter
  (`KismetSystemLibrary.Delay` 0.5)
  (`self.Possess` (`BlueprintMapLibrary.Map_Find` (`/Game/Blueprint/Global/Manager/BP_ComputerManager.DeskElement` (`self.Computer Manager`)) "NewEnumerator4"))
  (`self.ShowMouseCursor` false)
  (`WidgetBlueprintLibrary.SetInputMode_GameOnly` self))

(event `self.ReceivePossess`
  (params (PossessedPawn :type "Pawn Object Reference"))
  ;[1 1 1] hangement de pawn/ Ajouté condition d'ou on viens pour aller la ou on veux
  ;;[1 1 1] Comment
  ;;;[1 1 1] Possess Desk Element
  ;;;;[1 1 1] Possess event System
  (`self.PossessEvent` PossessedPawn))

(event `SetPossessTransistion`
  (params (PawnPossessed :type "Pawn Object Reference"))
  ;[1 1 1] hangement de pawn/ Ajouté condition d'ou on viens pour aller la ou on veux
  ;;[1 1 1] Comment
  ;;;[1 1 1] Possess Desk Element
  ;;;;[1 1 1] Transition Desk Element
  (`self.SetViewTargetWithBlend` PawnPossessed 0.4 "VTBlend_EaseOut" 1.25))

(event `self.ReceiveUnPossess`
  (params (UnpossessedPawn :type "Pawn Object Reference"))
  ;[1 1 1] hangement de pawn/ Ajouté condition d'ou on viens pour aller la ou on veux
  ;;[1 1 1] Comment
  ;;;[1 1 1] Possess Desk Element
  ;;;;[1 1 1] UnPossess Event
  (`self.UnPossessEvent` UnpossessedPawn))

(event `EnhancedInput|/Game/Blueprint/Character/Input/Action/Debug/IA_ChangePawn`
  (params (ActionValue :type Boolean) (ElapsedSeconds :type "Float (double-precision)") (TriggeredSeconds :type "Float (double-precision)") (InputAction :type "InputAction Object Reference" :default "/Game/Blueprint/Character/Input/Action/Debug/IA_ChangePawn.IA_ChangePawn"))
  ;[1 1 1] hangement de pawn/ Ajouté condition d'ou on viens pour aller la ou on veux
  ;;[1 1 1] Comment
  ;;;[1 1 1] Possess CameraActor/PlayerCharacter
  ;;;;[1 1 1] Debug Possess CameraActor/PlayerCharacter
  (:`Started`
    (if (`self.bShowMouseCursor`)
      (`self.OnChangePossesPawn` "NewEnumerator4")
      (else
        (`self.OnChangePossesPawn` "NewEnumerator3")))))

(fn `AddMappingContext`
  (params (MappingContext :type "InputMappingContext Object Reference"))
  (`EnhancedInputSubsystemInterface.AddMappingContext` (subsystem `EnhancedInputLocalPlayerSubsystem`) MappingContext 0 (struct)))

(fn `BindAllEvent`
  (`self.BindChangePosses`))

(fn `FindOfficeElement`
  (params (Key :type "/Game/Data/Enumerator/Desk/EOfficeElement Enum (by ref)"))
  (returns (Value :type "Pawn Object Reference"))
  (return (`BlueprintMapLibrary.Map_Find` (`/Game/Blueprint/Global/Manager/BP_ComputerManager.DeskElement` (`self.Computer Manager`)) Key)))

(fn `Input Mapping Initiate`
  (for _array_element (`self.Mapping Context`)
    (`EnhancedInputSubsystemInterface.AddMappingContext` (subsystem `EnhancedInputLocalPlayerSubsystem`) _array_element 0 (struct))))

(fn `PossessEvent`
  (params (`Current Possessed Pawn` :type "Pawn Object Reference"))
  (locals (CurrentPossessedPawn :type "Pawn Object Reference"))
  (set `local.CurrentPossessedPawn` `Current Possessed Pawn`)
  (switch `/Game/Data/Enumerator/Desk/EOfficeElement` (`self.Current Office Element`)
    (:`NewEnumerator2`
      (bind _asbp_hubscreen (cast `/Game/Blueprint/Office/Screen/BP_HUBScreen` (`local.CurrentPossessedPawn`)))
      (`/Game/Blueprint/Office/Screen/BP_HUBScreen.DisplayHubWidget` _asbp_hubscreen)
      (`self.ShowMouseCursor` true))
    (:`NewEnumerator3`
      (`self.PossessCameraActor`))
    (:`NewEnumerator4`
      (`self.PossessPlayerCharacter`))))

(fn `RemoveMappingContext`
  (params (MappingContext :type "InputMappingContext Object Reference"))
  (`EnhancedInputSubsystemInterface.RemoveMappingContext` (subsystem `EnhancedInputLocalPlayerSubsystem`) MappingContext (struct)))

(fn `SetManagerVariable`
  (bind _scene_manager (`self.Scene Manager`))
  (set `self.Computer Manager` (`/Game/Blueprint/Global/Manager/BP_SceneManager.ComputerManager` _scene_manager))
  (set `self.UIManager` (`/Game/Blueprint/Global/Manager/BP_SceneManager.UIManager` _scene_manager)))

(fn `UnPossessEvent`
  (params (UnPossessPawn :type "Pawn Object Reference"))
  (bind _asbp_hubscreen (cast `/Game/Blueprint/Office/Screen/BP_HUBScreen` UnPossessPawn)
    (:`then`
      (`/Game/Blueprint/Office/Screen/BP_HUBScreen.RemoveHubWidget` _asbp_hubscreen))
    (:`CastFailed`
      (bind _asbp_camera_controller (cast `/Game/Blueprint/Camera/BP_CameraController` UnPossessPawn))
      (`/Game/Blueprint/Camera/BP_CameraController.RemoveCameraWidget` _asbp_camera_controller))))

(fn `UserConstructionScript`)